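; BP_敵人 is an enemy pawn that wanders, chases the player boy (BP_男孩) and attacks on arrival.
; From BeginPlay it moves to random reachable points near its mesh, pausing briefly after each successful move before picking another.
; When PawnSensing sees the boy, AIMoveTo chases him and, on success, plays an attack montage.
; A DoOnce and the 攻擊玩家 flag block repeat attacks and new chases until the montage completes.
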(event `self.ReceiveBeginPlay`
  ;[1 1 1] 注释
  (`|AIMoveTo` self (`NavigationSystemV1.K2_GetRandomReachablePointInRadius` (`SceneComponent.K2_GetComponentLocation` (`self.Mesh`)) 500.0 null null) null :!label _label
    (:`OnSuccess`
      (`KismetSystemLibrary.Delay` (`KismetMathLibrary.RandomFloatInRange` 1.0 2.0))
      (goto _label))))

(event `self.PawnSensing.OnSeePawn`
  (params (Pawn :type "Pawn Object Reference"))
  (if (not (`self.攻擊玩家`))
    (bind `_asbp_男孩` (cast `/Game/BP/BP_男孩` Pawn))
    (`|AIMoveTo` self (0.0 0.0 0.0) `_asbp_男孩`
      (:`OnSuccess`
        (`/Engine/EditorBlueprintResources/StandardMacros.DoOnce` false :!label _label_2
          (:`Completed`
            (`|PlayMontage` (`self.Mesh`) "/Game/敵人動作/b敵人攻擊.b敵人攻擊"
              (:`then`
                (set `self.攻擊玩家` true))
              (:`OnCompleted`
                (set `self.攻擊玩家` false)
                (goto _label_2 :!via `Reset`)))))))))

(fn `UserConstructionScript`)