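; Player character Blueprint for an action game where the boy fights BP_敵人 enemies and collects BP_道具 items, winning at ten pickups.
; Input drives movement, sprinting, montage-timed weapon swapping between back and hand, and alternating light/heavy attacks gated by DoOnce.
; The weapon's overlap, switchable by function, damages enemies, while 受傷 lowers health clamped to 0–1.
; Death, polled on Tick, or victory shows an end widget and enables level restart.
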(event `InputAxis|MoveForward` :overrideparent false
  (params (AxisValue :type "Float (single-precision)"))
  ;[1 1 1] 移動
  (if (`self.是否死亡`)
    _
    (elif (`self.能否移動`)
      (`self.AddMovementInput` (`KismetMathLibrary.GetForwardVector` (`KismetMathLibrary.MakeRotator` 0.0 0.0 (.yaw (`self.GetControlRotation`)))) AxisValue))))

(event `InputAxis|Turn` :overrideparent false
  (params (AxisValue :type "Float (single-precision)"))
  ;[1 1 1] 滑鼠移動
  (`self.AddControllerYawInput` AxisValue))

(event `InputAxis|LookUp` :overrideparent false
  (params (AxisValue :type "Float (single-precision)"))
  ;[1 1 1] 滑鼠移動
  (`self.AddControllerPitchInput` AxisValue))

(event `InputAxis|MoveRight` :overrideparent false
  (params (AxisValue :type "Float (single-precision)"))
  ;[1 1 1] 移動
  (if (`self.是否死亡`)
    _
    (elif (`self.能否移動`)
      (`self.AddMovementInput` (`KismetMathLibrary.GetRightVector` (`KismetMathLibrary.MakeRotator` 0.0 0.0 (.yaw (`self.GetControlRotation`)))) AxisValue))))

(event `InputAction|衝刺`
  (params (Key :type "Key Structure"))
  (bind _charactermovement (`self.CharacterMovement`))
  ;[1 1 1] 衝刺跑步
  (:`Pressed`
    (set `CharacterMovementComponent.MaxWalkSpeed` 1200.0 _charactermovement))
  (:`Released`
    (set `CharacterMovementComponent.MaxWalkSpeed` 600.0 _charactermovement)))

(event `InputAction|更換武器`
  (params (Key :type "Key Structure"))
  (bind `_武器` (`self.武器`))
  ;[1 1 1] 拿武器
  (:`Pressed`
    (if (not (`self.是否死亡`))
      (set `self.更換武器` (not (`self.更換武器`)))
      (`|PlayMontage` (`self.Mesh`) "/Game/動作/拿武器_Montage.拿武器_Montage"
        (:`then`
          (if (`self.更換武器`)
            (`KismetSystemLibrary.Delay` 0.8)
            (`SceneComponent.K2_AttachToComponent` `_武器` (`self.右手`) "None" "KeepRelative" "KeepRelative" "KeepRelative" true)
            (else
              (`KismetSystemLibrary.Delay` 0.5)
              (`SceneComponent.K2_AttachToComponent` `_武器` (`self.背部`) "None" "KeepRelative" "KeepRelative" "KeepRelative" true)))
          (`KismetSystemLibrary.MoveComponentTo` `_武器` (0.0 0.0 0.0) (struct) false false 0.3))))))

(event `InputAction|輕攻擊`
  (params (Key :type "Key Structure"))
  ;[1 1 1] 輕攻擊
  (:`Pressed`
    (if (not (`self.是否死亡`))
      (`/Engine/EditorBlueprintResources/StandardMacros.DoOnce` false :!label _label
        (:`Completed`
          (if (`self.更換武器`)
            (`|PlayMontage` (`self.Mesh`) (select `int` (mod (`self.輕攻擊次數`) 2) :`0` "/Game/動作/第一段攻擊_Montage.第一段攻擊_Montage" :`1` "/Game/動作/第二段_Montage.第二段_Montage" :!type "AnimMontage Object Reference") 3.0
              (:`then`
                (`/Engine/EditorBlueprintResources/StandardMacros.IncrementInt` (`self.輕攻擊次數`)
                  (:`  `
                    (`KismetSystemLibrary.Delay` 0.1)
                    (if true
                      (`KismetSystemLibrary.Delay` 0.7)
                      (goto _label :!via `Reset`))))))
            (else
              (goto _label :!via `Reset`))))))))

(event `InputAction|重攻擊`
  (params (Key :type "Key Structure"))
  ;[1 1 1] 重攻擊
  (:`Pressed`
    (if (not (`self.是否死亡`))
      (`/Engine/EditorBlueprintResources/StandardMacros.DoOnce` false :!label _label_2
        (:`Completed`
          (if (`self.更換武器`)
            (`|PlayMontage` (`self.Mesh`) (select `int` (mod (`self.重攻擊次數`) 2) :`0` "/Game/動作/重攻擊1_Montage.重攻擊1_Montage" :`1` "/Game/動作/重攻擊2_Montage.重攻擊2_Montage" :!type "AnimMontage Object Reference") 1.5
              (:`then`
                (`/Engine/EditorBlueprintResources/StandardMacros.IncrementInt` (`self.重攻擊次數`)
                  (:`  `
                    (`KismetSystemLibrary.Delay` 0.5)
                    (if true
                      (`KismetSystemLibrary.Delay` 0.2)
                      (goto _label_2 :!via `Reset`))))))
            (else
              (goto _label_2 :!via `Reset`))))))))

(event `self.ReceiveBeginPlay`
  ;[1 1 1] 開始出現界面
  (bind _returnvalue (`|CreateWidget` "/Game/介面/介面.介面_C" (`GameplayStatics.GetPlayerController` 0)))
  (`UserWidget.AddToViewport` _returnvalue 0))

(event `self.武器碰撞.OnComponentBeginOverlap`
  (params (OverlappedComponent :type "PrimitiveComponent Object Reference") (OtherActor :type "Actor Object Reference") (OtherComp :type "PrimitiveComponent Object Reference") (OtherBodyIndex :type Integer) (bFromSweep :type Boolean) (SweepResult :type "HitResult Structure (by ref)"))
  ;[1 1 1] 被打
  (bind `_asbp_敵人` (cast `/Game/BP/BP_敵人` OtherActor))
  (`/Game/BP/BP_敵人.受傷` `_asbp_敵人` 30.0))

(event `self.CapsuleComponent.OnComponentBeginOverlap`
  (params (OverlappedComponent :type "PrimitiveComponent Object Reference") (OtherActor :type "Actor Object Reference") (OtherComp :type "PrimitiveComponent Object Reference") (OtherBodyIndex :type Integer) (bFromSweep :type Boolean) (SweepResult :type "HitResult Structure (by ref)"))
  (bind `_喇吧` (`self.喇吧`))
  ;[1 1 1] 道具音效
  (bind `_asbp_道具` (cast `/Game/BP/BP_道具` OtherActor))
  (`AudioComponent.SetSound` `_喇吧` "/Game/音效/Pickup_Coin7.Pickup_Coin7")
  (`AudioComponent.Play` `_喇吧` 0.0)
  (`self.K2_DestroyActor` `_asbp_道具`)
  (bind _result (`/Engine/EditorBlueprintResources/StandardMacros.IncrementInt` (`self.道具數量`))
    (:`  `
      (if (== _result 10)
        (`self.過關結束畫面` 0.5 "過關了")))))

(event `self.ReceiveTick`
  (params (DeltaSeconds :type "Float (single-precision)"))
  ;[1 1 1] 血量變0
  (if (`self.是否死亡`)
    (`/Engine/EditorBlueprintResources/StandardMacros.DoOnce` false
      (:`Completed`
        (`SkeletalMeshComponent.PlayAnimation` (`self.Mesh`) "/Game/動作/玩家死亡_Montage.玩家死亡_Montage" false)
        (`KismetSystemLibrary.Delay` 2.5)
        (`SkeletalMeshComponent.SetPlayRate` (`self.Mesh`) 0.0)
        (`self.過關結束畫面` 1.5 "失敗了...笑你W")))))

(event `InputAction|重新遊玩`
  (params (Key :type "Key Structure"))
  (:`Pressed`
    (if (`self.是否重新遊戲`)
      (`GameplayStatics.OpenLevel` "地圖"))))

(fn `UserConstructionScript`)

(fn `切換武器碰撞區域`
  (params (`是否顯示武器碰撞區域` :type Boolean))
  (set `PrimitiveComponent.bGenerateOverlapEvents` `是否顯示武器碰撞區域` (`self.武器碰撞`)))

(fn `切換移動`
  (params (`能否移動` :type Boolean))
  (set `self.能否移動` `能否移動`))

(fn `受傷`
  (params (`敵人傷害` :type "Float (double-precision)"))
  (if (`self.是否重新遊戲`)
    _
    (elif (not (`self.是否死亡`))
      (set `self.血量` (`KismetMathLibrary.FClamp` (- (`self.血量`) `敵人傷害`)))
      (`self.PlayAnimMontage` self "/Game/動作/玩家被打_Montage.玩家被打_Montage" 1.8 "None")
      (if (<= (`self.血量`) 0.0)
        (set `self.是否死亡` true)))))